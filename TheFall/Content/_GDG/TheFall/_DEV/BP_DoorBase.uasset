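; Base interactable door actor that swings open and closed, with an "Open" or "Close" prompt matching its state.
; Interact toggles IsOpen and plays or reverses the DoorRotation timeline, which drives the Door component's relative yaw.
; UpdatefromSave snaps the door straight to its open or closed angle from IsOpen, skipping the animation.
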(event `InteractionInterface.Interact`
  (params (Caller :type "TFCharacter Object Reference"))
  (bind _output_get (set `self.bIsOpen` (not (`self.bIsOpen`))))
  (if _output_get
    (bind (_direction _zrotation) (`Timeline|DoorRotation` :!label _label)
      (:`Update`
        (`SceneComponent.K2_SetRelativeRotation` (`self.Door`) (`KismetMathLibrary.MakeRotator` 0.0 0.0 _zrotation) false false)))
    (else
      (goto _label :!via `Reverse`))))

(event `SaveActorInterface.UpdateFromSave`
  (`SceneComponent.K2_SetRelativeRotation` (`self.Door`) (`KismetMathLibrary.MakeRotator` 0.0 0.0 (`KismetMathLibrary.SelectFloat` 110.0 0.0 (`self.bIsOpen`))) false false))

(fn `GetInteractionText`
  (returns (ReturnValue :type Text))
  (return (select `bool` (`self.bIsOpen`) :`false` "Open" :`true` "Close" :!type "Text")))

(fn `IsInteracable`
  (returns (ReturnValue :type Boolean))
  (return true))

(fn `UserConstructionScript`)